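; Dice-thrower cube that, on touch, spawns two Dado_BP dice above itself and launches them with random impulses after a short delay.
; Tick watches the dice until every velocity is near zero, then GetCaraSuperior finds each die's highest marker sphere and maps its index to face values 1–6.
; Results are written into the third-person character's ValorDados array and printed; the dice list and write index are never reset here.
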(event `self.ReceiveBeginPlay`
  (bind _asbp_third_person_character (cast `/Game/ThirdPerson/Blueprints/BP_ThirdPersonCharacter` (`GameplayStatics.GetPlayerCharacter` 0)))
  (set `self.Jugador` _asbp_third_person_character))

(event `self.ReceiveTick`
  (params (DeltaSeconds :type "Float (single-precision)"))
  (if (`self.DadoRodando`)
    (for _array_element (`self.VectorDado`)
      (if (== (`SceneComponent.GetComponentVelocity` (`/Game/Dado/Dado_BP.Dado` _array_element)) (0.0 0.0 0.0) :`ErrorTolerance` 0.0001)
        (set `self.DadoStop` true)
        (else
          (set `self.DadoStop` false)
          (break))))
    (if (`self.DadoStop`)
      (`KismetSystemLibrary.PrintText` "Los dados se detuvieron")
      (set `self.DadoRodando` false)
      (`self.GetCaraSuperior`))))

(event `self.Cube.OnInputTouchBegin`
  (params (FingerIndex :type "ETouchIndex Enum" :default "Touch1") (TouchedComponent :type "PrimitiveComponent Object Reference"))
  (bind _returnvalue (`|SpawnActorFromClass` "/Game/Dado/Dado_BP.Dado_BP_C" (`KismetMathLibrary.MakeTransform` (`KismetMathLibrary.MakeVector` (.x (`SceneComponent.K2_GetComponentLocation` (`self.Cube`))) (.y (`SceneComponent.K2_GetComponentLocation` (`self.Cube`))) (+ (.z (`SceneComponent.K2_GetComponentLocation` (`self.Cube`))) 200.0)) (struct) (0.3 0.3 0.3)) "Undefined" "OverrideRootScale" null null))
  (`KismetArrayLibrary.Array_Add` (`self.VectorDado`))
  (bind _returnvalue_2 (`|SpawnActorFromClass` "/Game/Dado/Dado_BP.Dado_BP_C" (`KismetMathLibrary.MakeTransform` (`KismetMathLibrary.MakeVector` (+ (.x (`SceneComponent.K2_GetComponentLocation` (`self.Cube`))) 75.0) (.y (`SceneComponent.K2_GetComponentLocation` (`self.Cube`))) (+ (.z (`SceneComponent.K2_GetComponentLocation` (`self.Cube`))) 200.0)) (struct) (0.3 0.3 0.3)) "Undefined" "OverrideRootScale" null null))
  (`KismetArrayLibrary.Array_Add` (`self.VectorDado`) _returnvalue_2)
  (`KismetSystemLibrary.Delay` 2.0)
  (`PrimitiveComponent.AddImpulse` (`/Game/Dado/Dado_BP.Dado` _returnvalue) (`KismetMathLibrary.MakeVector` (`KismetMathLibrary.RandomFloatInRange` -500.0 1500.0) (`KismetMathLibrary.RandomFloatInRange` -500.0 1500.0) (`KismetMathLibrary.RandomFloatInRange` 1000.0 1500.0)) "None" true)
  (`PrimitiveComponent.AddImpulse` (`/Game/Dado/Dado_BP.Dado` _returnvalue_2) (`KismetMathLibrary.MakeVector` (`KismetMathLibrary.RandomFloatInRange` -500.0 1500.0) (`KismetMathLibrary.RandomFloatInRange` -500.0 1500.0) (`KismetMathLibrary.RandomFloatInRange` 1000.0 1500.0)) "None" true)
  (`KismetSystemLibrary.Delay` 0.2)
  (set `self.DadoRodando` true)
  (set `self.DadoStop` false))

(fn `GetCaraSuperior`
  (for _array_element (`self.VectorDado`)
    (set `self.Eje_Z` -100.0)
    (for (_array_element_2 _array_index) (`/Game/Dado/Dado_BP.VectorDeBolas` _array_element)
      (bind _z (.z (`SceneComponent.K2_GetComponentLocation` _array_element_2)))
      (if (> _z (`self.Eje_Z`))
        (set `self.Eje_Z` _z)
        (set `self.BolaAlta` _array_element_2)
        (set `self.Indice_Esfera` _array_index)))
    (switch `int` (`self.Indice_Esfera`)
      (:`0`
        (set `self.ValorDado` 1))
      (:`1`
        (set `self.ValorDado` 2))
      (:`2`
        (set `self.ValorDado` 3))
      (:`3`
        (set `self.ValorDado` 4))
      (:`4`
        (set `self.ValorDado` 5))
      (:`5`
        (set `self.ValorDado` 6)))
    (`KismetArrayLibrary.Array_Set` (`/Game/ThirdPerson/Blueprints/BP_ThirdPersonCharacter.ValorDados` (`self.Jugador`)) (`self.Iterador`) (`self.ValorDado`))
    (`/Engine/EditorBlueprintResources/StandardMacros.IncrementInt` (`self.Iterador`)))
  (`self.Imprimir Valores`))

(fn `Imprimir Valores`
  (for _array_element (`/Game/ThirdPerson/Blueprints/BP_ThirdPersonCharacter.ValorDados` (`self.Jugador`))
    (`KismetSystemLibrary.PrintText` (`KismetTextLibrary.Conv_IntToText` _array_element))))

(fn `UserConstructionScript`)